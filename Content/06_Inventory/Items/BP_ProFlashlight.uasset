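; Battery-powered flashlight inventory item that toggles a spotlight and cylinder mesh on Use, only switching on while charge remains.
; A looping one-second timer drains the battery while lit and clears the switch when empty, with OnRep_OnOff updating the visuals.
; With authority, each drain writes the charge into the owning character's selected inventory slot and reloads the inventory.
; Use sounds come from the item DataTable, relayed through server and client events.
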(event `self.SetBatteryLevel`
  (params (NewBatteryLevel :type Integer))
  (set `self.CurrentBattery` NewBatteryLevel))

(event `self.SetSwitch`
  (params (Setting :type Boolean))
  (set `self.OnOff` Setting))

(event `self.ReceiveBeginPlay`
  (`KismetSystemLibrary.K2_SetTimer` null "Set" 1.0 true))

(event `ServerSoundPlay`
  (params (Sound :type "SoundBase Object Reference"))
  (`self.ClientSoundPlay` Sound))

(event `self.Use`
  (if (`self.OnOff`)
    (set `self.OnOff` false)
    (`LightComponent.SetIntensity` (`self.SpotLight`) (`self.Off`))
    (`SceneComponent.SetVisibility` (`self.Cylinder`) false false)
    (bind _returnvalue (`|GetDataTableRow` "/Game/06_Inventory/ItemData/DT_ItemData.DT_ItemData" (`.RowName` (break `DataTableRowHandle` (`.ItemID` (break `Item` (`self.itemdata`))))) :!label _label)
      (:`then`
        (`self.ServerSoundPlay` (`.Use` (break `SFX` (`.SFX` (break `ItemData` _returnvalue)))))))
    (elif (> (`self.CurrentBattery`) 0)
      (set `self.OnOff` true)
      (`LightComponent.SetIntensity` (`self.SpotLight`) (`self.On`))
      (`SceneComponent.SetVisibility` (`self.Cylinder`) true false)
      (goto _label))))

(event `ClientSoundPlay`
  (params (Sound :type "SoundBase Object Reference"))
  (`GameplayStatics.PlaySoundAtLocation` Sound (`self.K2_GetActorLocation` (`self.GetOwner`)) (struct) 1.0 1.0 0.0 null null null null))

(event `Set`
  (bind _returnvalue (`self.GetOwner`))
  (if (and (> (`self.CurrentBattery`) 0) (`self.OnOff`))
    (bind _result (`/Engine/EditorBlueprintResources/StandardMacros.DecrementInt` (`self.CurrentBattery`))
      (:`  `
        (set `self.CurrentBattery` _result)
        (bind _asbp_third_person_character (cast `/Game/ThirdPerson/Blueprints/BP_ThirdPersonCharacter` _returnvalue))
        (if (`self.HasAuthority` _returnvalue)
          (`self.BatterySet`))))
    (else
      (set `self.OnOff` false))))

(event `BatterySet`
  (bind _inventorycomponent (`TP_ThirdPersonCharacter.InventoryComponent` (stale `Set` _asbp_third_person_character)))
  (bind _inventory (`InventoryComponent.Inventory` _inventorycomponent))
  (bind _selectinventory (`TP_ThirdPersonCharacter.SelectInventory` (stale `Set` _asbp_third_person_character)))
  (bind (_output_itemid _output_itemcount _output_maxbattery) (break `Item` (`|GetArrayItem` _inventory _selectinventory)))
  (`KismetArrayLibrary.Array_Set` _inventory _selectinventory (make `Item` _output_itemid _output_itemcount _output_maxbattery (`self.CurrentBattery`)))
  (`InventoryComponent.reloadinventory` _inventorycomponent))

(fn `GetBatteryLevel`
  (returns (ReturnValue :type Integer))
  (return (`self.CurrentBattery`)))

(fn `GetMaxBatteryLevel`
  (returns (ReturnValue :type Integer))
  (return (`self.MaxBattery`)))

(fn `GetSwitch`
  (returns (ReturnValue :type Boolean))
  (return (`self.OnOff`)))

(fn `OnRep_OnOff`
  (if (`self.OnOff`)
    (`LightComponent.SetIntensity` (`self.SpotLight`) (`self.On`))
    (`SceneComponent.SetVisibility` (`self.Cylinder`) true false)
    (else
      (`LightComponent.SetIntensity` (`self.SpotLight`) (`self.Off`))
      (`SceneComponent.SetVisibility` (`self.Cylinder`) false false))))

(fn `UserConstructionScript`)