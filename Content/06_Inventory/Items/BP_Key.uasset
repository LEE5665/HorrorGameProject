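; BP_Key is an inventory key item that unlocks a locked door when its owning third-person character uses it.
; Use line-traces a short distance forward from the owner's camera and casts the hit actor to BaseDoor.
; If that door is locked, it clears the lock, removes the selected inventory item without spawning a pickup, and plays a ping sound at the door.
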(event `self.Use`
  (bind _asbp_third_person_character (cast `/Game/ThirdPerson/Blueprints/BP_ThirdPersonCharacter` (`self.GetOwner`)))
  (bind _desiredview (`CameraComponent.GetCameraView` (`/Game/ThirdPerson/Blueprints/BP_ThirdPersonCharacter.Camera` _asbp_third_person_character) 0.0))
  (bind _outhit (`KismetSystemLibrary.LineTraceSingle` (break `MinimalViewInfo` _desiredview) (+ (break `MinimalViewInfo` _desiredview) (* (`KismetMathLibrary.GetForwardVector` (`.Rotation` (break `MinimalViewInfo` _desiredview))) 200.0)) "TraceTypeQuery3"))
  (bind _asbase_door (cast `BaseDoor` (`.HitActor` (`GameplayStatics.BreakHitResult` _outhit))))
  (if (`BaseDoor.isLock` _asbase_door)
    (set `BaseDoor.isLock` false _asbase_door)
    (`InventoryComponent.DropItem` (`TP_ThirdPersonCharacter.InventoryComponent` _asbp_third_person_character) (`TP_ThirdPersonCharacter.SelectInventory` _asbp_third_person_character) false)
    (`/Game/ThirdPerson/Blueprints/BP_ThirdPersonCharacter.PlaySound` _asbp_third_person_character "/Engine/EngineSounds/1kSineTonePing.1kSineTonePing" (`self.K2_GetActorLocation` _asbase_door))))

(fn `UserConstructionScript`)