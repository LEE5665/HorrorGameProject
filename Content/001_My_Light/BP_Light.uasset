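; BP_Light is a light Blueprint that makes a RectLight flicker between a minimum and maximum intensity.
; Tick calls FlickeringLight, which reapplies the light color every frame and, when IsFlickering is true, clears that flag and starts a timeline at a random play rate.
; The timeline's curve drives the intensity lerp, and its finish re-arms the flag, so cycles repeat at varying speeds.
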(event `self.ReceiveTick`
  (params (DeltaSeconds :type "Float (single-precision)"))
  (`self.FlickeringLight`))

(event `FlickeringLight`
  ;[0.04908 0.06149 0.08646] [Custom Event] FlickeringLight
  (`LightComponent.SetLightColor` (`self.RectLight`) (`self.LightColor`) true)
  (if (`self.IsFlickering?`)
    (`TimelineComponent.SetPlayRate` (`self.Timeline_Test`) (`KismetMathLibrary.RandomFloatInRange` (`self.FlickeringMinSpeed`) (`self.FlickeringMaxSpeed`)))
    (set `self.IsFlickering?` false)
    (bind (_direction _intensity) (`Timeline|Timeline_Test` :`NewTime` 5.0 :!via `PlayFromStart`)
      (:`Update`
        (`LightComponent.SetIntensity` (`self.RectLight`) (`KismetMathLibrary.Lerp` (`self.IntensityMin`) (`self.IntensityMax`) _intensity)))
      (:`Finished`
        (set `self.IsFlickering?` true)))))

(fn `UserConstructionScript`)