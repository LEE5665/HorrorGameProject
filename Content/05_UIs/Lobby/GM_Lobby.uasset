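; Lobby game mode that tracks player controllers, manages the save slot chosen in the game instance, and seamlessly travels to the hospital map.
; BeginPlay creates or loads BP_Save, with Day and Money crossed into GameMoney and GameDay on load.
; SaveInventory writes those values and each player's inventory, which InventoryMatching restores by matching TestName.
; TestNetIdSet assigns numbered test names as player IDs; the seamless-travel actor-list override is unfinished.
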(event `MapChange`
  (`KismetSystemLibrary.ExecuteConsoleCommand` "net.AllowPIESeamlessTravel 1" null)
  (set `self.bUseSeamlessTravel` true)
  (`AdvancedSessionsLibrary.ServerTravel` "/Game/00_Levels/Level/Map_Hospital"))

(event `TestNetIdSet`
  (params (PC :type "PlayerController Object Reference"))
  ;[1 1 1] 테스트 ID 설정
  (bind _asbp_third_person_character (cast `/Game/ThirdPerson/Blueprints/BP_ThirdPersonCharacter` (`Controller.K2_GetPawn` PC)))
  (set `/Game/ThirdPerson/Blueprints/BP_ThirdPersonCharacter.TestName` (`KismetStringLibrary.Concat_StrStr` "Player" (`KismetStringLibrary.Conv_IntToString` (`self.TestNumber`))) _asbp_third_person_character)
  (bind _result (`/Engine/EditorBlueprintResources/StandardMacros.IncrementInt` (`self.TestNumber`))
    (:`  `
      (set `self.TestNumber` _result))))

(event `self.ReceiveBeginPlay`
  ;[1 1 1] 세이브
  (bind _asbp_game_instance (cast `/Game/02_Blueprints/BP_GameInstance` (`GameplayStatics.GetGameInstance`)))
  (bind _returnvalue (`GameplayStatics.DoesSaveGameExist` (`KismetStringLibrary.Conv_IntToString` (`/Game/02_Blueprints/BP_GameInstance.SetSlot` _asbp_game_instance))))
  (if _returnvalue
    (bind _asbp_game_instance_2 (cast `/Game/02_Blueprints/BP_GameInstance` (`GameplayStatics.GetGameInstance`)))
    (bind _setslot (`/Game/02_Blueprints/BP_GameInstance.SetSlot` _asbp_game_instance_2))
    (bind _returnvalue_2 (`GameplayStatics.LoadGameFromSlot` (`KismetStringLibrary.Conv_IntToString` _setslot) _setslot))
    (bind _asbp_save (cast `/Game/02_Blueprints/BP_Save` _returnvalue_2))
    (set `self.GameMoney` (`/Game/02_Blueprints/BP_Save.Day` _asbp_save))
    (set `self.GameDay` (`/Game/02_Blueprints/BP_Save.Money` _asbp_save))
    (else
      (bind _returnvalue_3 (`GameplayStatics.CreateSaveGameObject` "/Game/02_Blueprints/BP_Save.BP_Save_C"))
      (set `/Game/02_Blueprints/BP_Save.Day` 0 _returnvalue_3)
      (set `/Game/02_Blueprints/BP_Save.Money` 0 _returnvalue_3)
      (bind _asbp_game_instance_3 (cast `/Game/02_Blueprints/BP_GameInstance` (`GameplayStatics.GetGameInstance`)))
      (`GameplayStatics.SaveGameToSlot` _returnvalue_3 (`KismetStringLibrary.Conv_IntToString` (`/Game/02_Blueprints/BP_GameInstance.SetSlot` _asbp_game_instance_3))))))

(event `self.K2_PostLogin`
  (params (NewPlayer :type "PlayerController Object Reference"))
  ;[1 1 1] 컨트롤러 할당
  (`KismetArrayLibrary.Array_Add` (`self.PCs`) NewPlayer))

(event `InventoryMatching`
  (params (PC :type "PlayerController Object Reference"))
  (bind _asbp_third_person_character (cast `/Game/ThirdPerson/Blueprints/BP_ThirdPersonCharacter` (`Controller.K2_GetPawn` PC)))
  (bind _asbp_game_instance (cast `/Game/02_Blueprints/BP_GameInstance` (`GameplayStatics.GetGameInstance`)))
  (bind _returnvalue (`GameplayStatics.LoadGameFromSlot` (`KismetStringLibrary.Conv_IntToString` (`/Game/02_Blueprints/BP_GameInstance.SetSlot` _asbp_game_instance))))
  (bind _asbp_save (cast `/Game/02_Blueprints/BP_Save` _returnvalue))
  (for _array_element (`/Game/02_Blueprints/BP_Save.PlayerData` _asbp_save)
    (if (`KismetStringLibrary.EqualEqual_StrStr` (break `/Game/05_UIs/Lobby/Struct/S_PlayerData` _array_element) (`/Game/ThirdPerson/Blueprints/BP_ThirdPersonCharacter.TestName` _asbp_third_person_character))
      (bind _inventorycomponent (`TP_ThirdPersonCharacter.InventoryComponent` _asbp_third_person_character))
      (set `InventoryComponent.Inventory` (`.Inventory_15_92D40F75488160BDD4B1D6AD2DFC5867` (break `/Game/05_UIs/Lobby/Struct/S_PlayerData` _array_element)) _inventorycomponent)
      (`KismetSystemLibrary.PrintString` "바꿈!")
      (`InventoryComponent.reloadinventory` _inventorycomponent))))

(event `self.K2_OnLogout`
  (params (ExitingController :type "Controller Object Reference"))
  ;[1 1 1] 컨트롤러 할당
  (bind _asplayer_controller (cast `PlayerController` ExitingController))
  (`KismetArrayLibrary.Array_RemoveItem` (`self.PCs`) _asplayer_controller))

(event `SaveInventory`
  (bind _returnvalue (`GameplayStatics.CreateSaveGameObject` "/Game/02_Blueprints/BP_Save.BP_Save_C"))
  (set `/Game/02_Blueprints/BP_Save.Day` (`self.GameDay`) _returnvalue)
  (set `/Game/02_Blueprints/BP_Save.Money` (`self.GameMoney`) _returnvalue)
  (for _array_element (`self.PCs`)
    (bind _asbp_third_person_character (cast `/Game/ThirdPerson/Blueprints/BP_ThirdPersonCharacter` (`Controller.K2_GetPawn` _array_element)))
    (bind _testname (`/Game/ThirdPerson/Blueprints/BP_ThirdPersonCharacter.TestName` _asbp_third_person_character))
    (`KismetSystemLibrary.PrintString` _testname)
    (`KismetArrayLibrary.Array_Add` (`/Game/02_Blueprints/BP_Save.PlayerData` _returnvalue) (make `/Game/05_UIs/Lobby/Struct/S_PlayerData` _testname (`InventoryComponent.Inventory` (`TP_ThirdPersonCharacter.InventoryComponent` _asbp_third_person_character)))))
  (bind _asbp_game_instance (cast `/Game/02_Blueprints/BP_GameInstance` (`GameplayStatics.GetGameInstance`)))
  (`GameplayStatics.SaveGameToSlot` _returnvalue (`KismetStringLibrary.Conv_IntToString` (`/Game/02_Blueprints/BP_GameInstance.SetSlot` _asbp_game_instance)))
  (`KismetSystemLibrary.PrintString` "저장!"))

(fn `K2_OnGetSeamlessTravelActorList`
  (params (bToTransitionOut :type Boolean) (ActorListOut :type "Array of Actor Object Reference (by ref)"))
  (returns (ReturnValue :type "Array of Actor Object Reference")))

(fn `UserConstructionScript`)