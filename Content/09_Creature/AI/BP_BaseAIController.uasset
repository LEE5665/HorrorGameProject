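; Base AI controller for creatures that runs BT_BaseAI and tracks the player character through AI Perception.
; Perception updates write any BP_ThirdPersonCharacter to the Enemy blackboard key and set isEnemy, without checking whether it was gained or lost.
; Each update resets a timer, restarted only when sight perceives no actors; its expiry clears isEnemy but leaves Enemy set, giving a short memory after losing sight.
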(event `self.ReceiveBeginPlay`
  (`self.RunBehaviorTree` "/Game/09_Creature/AI/BT_BaseAI.BT_BaseAI"))

(event `self.AIPerception.OnPerceptionUpdated`
  (params (UpdatedActors :type "Array of Actor Object Reference (by ref)"))
  (`|ExecutionSequence`
    (:`then_0`
      (for _array_element UpdatedActors
        (bind _asbp_third_person_character (cast `/Game/ThirdPerson/Blueprints/BP_ThirdPersonCharacter` _array_element))
        (`BlackboardComponent.SetValueAsObject` (`AIBlueprintHelperLibrary.GetBlackboard` null) "Enemy" _asbp_third_person_character)
        (`BlackboardComponent.SetValueAsBool` (`AIBlueprintHelperLibrary.GetBlackboard` null) "isEnemy" true)))
    (:`then_1`
      (`KismetSystemLibrary.K2_ClearAndInvalidateTimerHandle` (`self.Timer`))
      (if (== (`KismetArrayLibrary.Array_Length` (`AIPerceptionComponent.GetCurrentlyPerceivedActors` (`self.AIPerception`) "/Script/AIModule.AISense_Sight")) 0)
        (bind _returnvalue (`KismetSystemLibrary.K2_SetTimerDelegate` (delegate `Null`) 5.0))
        (set `self.Timer` _returnvalue)))))

(event `Null`
  (`KismetSystemLibrary.PrintString` "잃어버림")
  (`BlackboardComponent.SetValueAsBool` (`AIBlueprintHelperLibrary.GetBlackboard` null) "isEnemy" false))

(fn `UserConstructionScript`)