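; Teleport zone actor that counts player characters inside its Box and shows current and max counts on a WB_TeleportDisplay widget.
; On overlap begin or end, it recounts overlapping BP_ThirdPersonCharacters and passes the total to the triggering character's ServerPlayerCount.
; RepNotifies on CurrentCount and MaxCount push replicated values into the widget and refresh its text.
; The construction script sizes the Box from Scale; the teleport itself is not handled here.
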(event `self.ReceiveBeginPlay`
  (bind _aswb_teleport_display (cast `/Game/02_Blueprints/MapBlueprint/WB_TeleportDisplay` (`WidgetComponent.GetUserWidgetObject` (`self.Widget`))))
  (`/Game/02_Blueprints/MapBlueprint/WB_TeleportDisplay.TextChange` _aswb_teleport_display))

(event `self.Box.OnComponentBeginOverlap`
  (params (OverlappedComponent :type "PrimitiveComponent Object Reference") (OtherActor :type "Actor Object Reference") (OtherComp :type "PrimitiveComponent Object Reference") (OtherBodyIndex :type Integer) (bFromSweep :type Boolean) (SweepResult :type "HitResult Structure (by ref)"))
  (bind _asbp_third_person_character (cast `/Game/ThirdPerson/Blueprints/BP_ThirdPersonCharacter` OtherActor))
  (set `self.Count` 0)
  (for _ (`PrimitiveComponent.GetOverlappingActors` (`self.Box`) "/Game/ThirdPerson/Blueprints/BP_ThirdPersonCharacter.BP_ThirdPersonCharacter_C")
    (bind _result (`/Engine/EditorBlueprintResources/StandardMacros.IncrementInt` (`self.Count`))
      (:`  `
        (bind _output_get (set `self.Count` _result)))))
  (`/Game/ThirdPerson/Blueprints/BP_ThirdPersonCharacter.ServerPlayerCount` _asbp_third_person_character _output_get))

(event `self.Box.OnComponentEndOverlap`
  (params (OverlappedComponent :type "PrimitiveComponent Object Reference") (OtherActor :type "Actor Object Reference") (OtherComp :type "PrimitiveComponent Object Reference") (OtherBodyIndex :type Integer))
  (bind _asbp_third_person_character (cast `/Game/ThirdPerson/Blueprints/BP_ThirdPersonCharacter` OtherActor))
  (set `self.Count` 0)
  (for _ (`PrimitiveComponent.GetOverlappingActors` (`self.Box`) "/Game/ThirdPerson/Blueprints/BP_ThirdPersonCharacter.BP_ThirdPersonCharacter_C")
    (bind _result (`/Engine/EditorBlueprintResources/StandardMacros.IncrementInt` (`self.Count`))
      (:`  `
        (bind _output_get (set `self.Count` _result)))))
  (`/Game/ThirdPerson/Blueprints/BP_ThirdPersonCharacter.ServerPlayerCount` _asbp_third_person_character _output_get))

(fn `OnRep_CurrentCount`
  (bind _aswb_teleport_display (cast `/Game/02_Blueprints/MapBlueprint/WB_TeleportDisplay` (`WidgetComponent.GetUserWidgetObject` (`self.Widget`))))
  (set `/Game/02_Blueprints/MapBlueprint/WB_TeleportDisplay.CurrentCount` (`self.CurrentCount`) _aswb_teleport_display)
  (`/Game/02_Blueprints/MapBlueprint/WB_TeleportDisplay.TextChange` _aswb_teleport_display))

(fn `OnRep_MaxCount`
  (bind _aswb_teleport_display (cast `/Game/02_Blueprints/MapBlueprint/WB_TeleportDisplay` (`WidgetComponent.GetUserWidgetObject` (`self.Widget`))))
  (set `/Game/02_Blueprints/MapBlueprint/WB_TeleportDisplay.MaxCount` (`self.MaxCount`) _aswb_teleport_display)
  (`/Game/02_Blueprints/MapBlueprint/WB_TeleportDisplay.TextChange` _aswb_teleport_display))

(fn `PlayerCount`)

(fn `UserConstructionScript`
  (`SceneComponent.SetWorldScale3D` (`self.Box`) (`self.Scale`)))