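; BP_Display is a lobby display actor that shows replicated teleport and money information on a widget component.
; RepNotify functions for current count, max count, map index and money cast the widget to WB_TeleportDisplay or WB_Display and refresh it, though current count and map index pass a constant zero.
; The construction script sizes and recenters the Box, whose overlap events are empty, leaving the server-side player counting logic disconnected.
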(event `self.ReceiveBeginPlay`)

(event `self.Box.OnComponentBeginOverlap`
  (params (OverlappedComponent :type "PrimitiveComponent Object Reference") (OtherActor :type "Actor Object Reference") (OtherComp :type "PrimitiveComponent Object Reference") (OtherBodyIndex :type Integer) (bFromSweep :type Boolean) (SweepResult :type "HitResult Structure (by ref)")))

(event `self.Box.OnComponentEndOverlap`
  (params (OverlappedComponent :type "PrimitiveComponent Object Reference") (OtherActor :type "Actor Object Reference") (OtherComp :type "PrimitiveComponent Object Reference") (OtherBodyIndex :type Integer)))

(fn `OnRep_CurrentCount`
  (bind _aswb_teleport_display (cast `/Game/02_Blueprints/MapBlueprint/LobbyDisplay/WB_TeleportDisplay` (`WidgetComponent.GetUserWidgetObject` (`self.Widget`))))
  (set `/Game/02_Blueprints/MapBlueprint/LobbyDisplay/WB_TeleportDisplay.CurrentCount` 0 _aswb_teleport_display)
  (`/Game/02_Blueprints/MapBlueprint/LobbyDisplay/WB_TeleportDisplay.TextChange` _aswb_teleport_display))

(fn `OnRep_MapIndex`
  (bind _aswb_teleport_display (cast `/Game/02_Blueprints/MapBlueprint/LobbyDisplay/WB_TeleportDisplay` (`WidgetComponent.GetUserWidgetObject` (`self.Widget`))))
  (set `/Game/02_Blueprints/MapBlueprint/LobbyDisplay/WB_TeleportDisplay.MapIndex` 0 _aswb_teleport_display)
  (`/Game/02_Blueprints/MapBlueprint/LobbyDisplay/WB_TeleportDisplay.MapChange` _aswb_teleport_display))

(fn `OnRep_MaxCount`
  (bind _aswb_teleport_display (cast `/Game/02_Blueprints/MapBlueprint/LobbyDisplay/WB_TeleportDisplay` (`WidgetComponent.GetUserWidgetObject` (`self.Widget`))))
  (set `/Game/02_Blueprints/MapBlueprint/LobbyDisplay/WB_TeleportDisplay.MaxCount` (`self.MaxCount`) _aswb_teleport_display)
  (`/Game/02_Blueprints/MapBlueprint/LobbyDisplay/WB_TeleportDisplay.TextChange` _aswb_teleport_display))

(fn `OnRep_Money`
  (bind _aswb_display (cast `/Game/02_Blueprints/MapBlueprint/LobbyDisplay/WB_Display` (`WidgetComponent.GetUserWidgetObject` (`self.Widget`))))
  (set `/Game/02_Blueprints/MapBlueprint/LobbyDisplay/WB_Display.Money` (`self.Money`) _aswb_display)
  (`/Game/02_Blueprints/MapBlueprint/LobbyDisplay/WB_Display.ChangeText` _aswb_display))

(fn `UserConstructionScript`
  (`SceneComponent.SetWorldScale3D` (`self.Box`) (`self.Scale`))
  (`SceneComponent.K2_SetRelativeLocation` (`self.Box`) (0.0 0.0 0.0) false false))