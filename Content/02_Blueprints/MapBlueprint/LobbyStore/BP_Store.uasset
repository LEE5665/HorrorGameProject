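; BP_Store is a lobby store actor that shows money, the selected item and the current tab on a WB_StoreDisplay widget.
; On BeginPlay the server sets its owner to each BP_ThirdPersonCharacter in turn and calls ServerDisplayMoneyInit on GM_Lobby inside that loop.
; RepNotify functions for Money, StoreSelectedItem and TabIndex copy each value into the widget and trigger its refresh.
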(event `self.ReceiveBeginPlay`
  (if (`self.HasAuthority`)
    (bind _outactors (`GameplayStatics.GetAllActorsOfClass` "/Game/ThirdPerson/Blueprints/BP_ThirdPersonCharacter.BP_ThirdPersonCharacter_C"))
    (for _array_element _outactors
      (`self.SetOwner` _array_element)
      (bind _asgm_lobby (cast `/Game/05_UIs/Lobby/GM_Lobby` (`GameplayStatics.GetGameMode`)))
      (`/Game/05_UIs/Lobby/GM_Lobby.ServerDisplayMoneyInit` _asgm_lobby))))

(fn `OnRep_Money`
  (bind _aswb_store_display (cast `/Game/02_Blueprints/MapBlueprint/LobbyStore/WB_StoreDisplay` (`WidgetComponent.GetUserWidgetObject` (`self.Widget`))))
  (set `/Game/02_Blueprints/MapBlueprint/LobbyStore/WB_StoreDisplay.Money` (`self.Money`) _aswb_store_display)
  (`/Game/02_Blueprints/MapBlueprint/LobbyStore/WB_StoreDisplay.MoneyUpdate` _aswb_store_display))

(fn `OnRep_StoreSelectedItem`
  (bind _aswb_store_display (cast `/Game/02_Blueprints/MapBlueprint/LobbyStore/WB_StoreDisplay` (`WidgetComponent.GetUserWidgetObject` (`self.Widget`))))
  (set `/Game/02_Blueprints/MapBlueprint/LobbyStore/WB_StoreDisplay.Item` (`self.StoreSelectedItem`) _aswb_store_display)
  (`/Game/02_Blueprints/MapBlueprint/LobbyStore/WB_StoreDisplay.ItemUpdate` _aswb_store_display))

(fn `OnRep_TabIndex`
  (bind _aswb_store_display (cast `/Game/02_Blueprints/MapBlueprint/LobbyStore/WB_StoreDisplay` (`WidgetComponent.GetUserWidgetObject` (`self.Widget`))))
  (set `/Game/02_Blueprints/MapBlueprint/LobbyStore/WB_StoreDisplay.TabIndex` (`self.TabIndex`) _aswb_store_display)
  (`/Game/02_Blueprints/MapBlueprint/LobbyStore/WB_StoreDisplay.TabUpdate` _aswb_store_display)
  (`/Game/02_Blueprints/MapBlueprint/LobbyStore/WB_StoreDisplay.TabColor` _aswb_store_display))

(fn `UserConstructionScript`)