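; GM_AllLevel is a game mode that handles game over and travel back to the lobby.
; GameOverEvent runs once, shows the game over widget to spectators' controllers, then after a delay deletes the current save slot and clears player state inventories.
; It then calls MapChange, which enables seamless travel and always server-travels to Map_Lobby, ignoring its map name argument.
; Random navmesh flashlight spawning is present but never runs.
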(event `MapChange`
  (params (TravelMapName :type String))
  (`KismetSystemLibrary.ExecuteConsoleCommand` "net.AllowPIESeamlessTravel 1" null)
  (set `self.bUseSeamlessTravel` true)
  (`AdvancedSessionsLibrary.ServerTravel` "/Game/00_Levels/Map_Lobby"))

(event `GameOverEvent`
  (if (not (`self.GameOver`))
    (set `self.GameOver` true)
    (bind _outactors (`GameplayStatics.GetAllActorsOfClass` "/Game/ThirdPerson/Blueprints/BP_Spectator.BP_Spectator_C"))
    (for _array_element _outactors
      (bind _asbp_player_controller (cast `/Game/02_Blueprints/Player/BP_PlayerController` (`Pawn.GetController` _array_element)))
      (`/Game/02_Blueprints/Player/BP_PlayerController.GameOverWidget` _asbp_player_controller))
    (`KismetSystemLibrary.Delay` 5.0)
    (bind _asbp_game_instance (cast `/Game/02_Blueprints/BP_GameInstance` (`GameplayStatics.GetGameInstance`)))
    (`GameplayStatics.DeleteGameInSlot` (`KismetStringLibrary.Conv_IntToString` (`/Game/02_Blueprints/BP_GameInstance.SetSlot` _asbp_game_instance)))
    (bind _outactors_2 (`GameplayStatics.GetAllActorsOfClass` "/Game/02_Blueprints/Player/BP_PlayerState.BP_PlayerState_C"))
    (for _array_element_2 _outactors_2
      (`KismetArrayLibrary.Array_Clear` (`/Game/02_Blueprints/Player/BP_PlayerState.inventory` _array_element_2)))
    (`self.MapChange` "")))

(event `self.ReceiveBeginPlay`)

(fn `NewFunction`)

(fn `UserConstructionScript`)